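; Base enemy Blueprint with health, an overhead-style health bar widget, damage over time and ragdoll death.
; BPC_CharacterInfo refills health on BeginPlay, and its death event disables capsule collision and switches the mesh to physics simulation.
; Each health change updates the W_HealBarEnemy widget and sets a one-second timer, looping if TimerDoT is non-zero.
; That timer subtracts fixed health and decrements TimerDoT while DamageOverTime is active and ticks remain, printing the count.
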(event OnDeath(BPC_CharacterInfo)
  (bind _mesh (Variables|Character|GetMesh))
  (Collision|SetCollisionEnabled (Variables|Collision|GetCapsuleComponent) "NoCollision")
  (Collision|SetCollisionProfileName _mesh "PhysicsActor" true :!class /Script/Engine.PrimitiveComponent)
  (Physics|SetSimulatePhysics _mesh true))

(event OnHealthChange(BPC_CharacterInfo)
  (params (CurrentHealth :type Float%20%28double-precision%29) (MaxHealth :type Float%20%28double-precision%29))
  (Utilities|Time|SetTimerbyEvent (delegate Custom|AppyDoT) 1.0 (Math|Conversions|ToBoolean(Integer) (Variables|Default|GetTimerDoT)))
  (bind _asw_heal_bar_enemy (Utilities|Casting|CastToW_HealBarEnemy (UserInterface|GetUserWidgetObject (Variables|Default|GetHealthWidget))))
  (Variables|Default|SetAs%20W%20Heal%20Bar%20Enemy _asw_heal_bar_enemy)
  (Default|SetNewHealth (Variables|Default|GetAs%20W%20Heal%20Bar%20Enemy) (Variables|/Game/ARpgFps/Characters/Global/BPC_CharacterInfo.BPC_CharacterInfo_C|GetHealth (Variables|Default|GetBPC_CharacterInfo)) (Variables|/Game/ARpgFps/Characters/Global/BPC_CharacterInfo.BPC_CharacterInfo_C|GetMaxHealth (Variables|Default|GetBPC_CharacterInfo))))

(event Custom|AppyDoT
  (if (and (Variables|Default|GetDamageOverTime) (> (Variables|Default|GetTimerDoT) 0))
    (Default|SetHealth (Variables|Default|GetBPC_CharacterInfo) (- (Variables|/Game/ARpgFps/Characters/Global/BPC_CharacterInfo.BPC_CharacterInfo_C|GetHealth (Variables|Default|GetBPC_CharacterInfo)) 5.0))
    (Variables|Default|SetTimerDoT (- (Variables|Default|GetTimerDoT) 1))
    (Development|PrintString (Utilities|String|ToString(Integer) (Variables|Default|GetTimerDoT)))))

(event EventBeginPlay
  (Default|ReFillHealth (Variables|Default|GetBPC_CharacterInfo)))

(fn ConstructionScript)