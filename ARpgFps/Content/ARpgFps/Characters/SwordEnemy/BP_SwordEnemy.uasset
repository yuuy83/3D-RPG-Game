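; BP_SwordEnemy is a sword enemy character for the ARpgFps game, and its own logic covers death.
; When BPC_CharacterInfo fires OnDeath, it stops the AI controller's brain logic, disables capsule collision and turns the mesh into a physics ragdoll.
; The actor is destroyed after a short delay.
; BeginPlay only calls the parent, and a leftover SetHealth node is never executed.
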(event OnDeath(BPC_CharacterInfo)
  (bind _mesh (Variables|Character|GetMesh))
  (Utilities|FlowControl|Sequence
    (:then_0
      (AI|Logic|StopLogic (Variables|/Script/AIModule.AIController|GetBrainComponent (AI|GetAIController self)) "Death"))
    (:then_1
      (Collision|SetCollisionEnabled (Variables|Default|GetCapsuleComponent) "NoCollision")
      (Audio|Components|Audio|Stop _mesh)
      (Collision|SetCollisionProfileName _mesh "PhysicsActor" true :!class /Script/Engine.PrimitiveComponent)
      (Physics|SetSimulatePhysics _mesh true))
    (:then_2
      (Utilities|FlowControl|Delay 3.0)
      (Actor|DestroyActor))))

(event EventBeginPlay
  (|CallParentFunction))

(event Collision|EventActorBeginOverlap
  (params (OtherActor :type Actor%20Object%20Reference)))

(event EventTick
  (params (DeltaSeconds :type Float%20%28single-precision%29)))

(fn ConstructionScript
  (|CallParentFunction))