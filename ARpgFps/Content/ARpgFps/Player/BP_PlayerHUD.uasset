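; Player HUD Blueprint that puts the WBP_HUD widget on screen at BeginPlay.
; It creates the widget, stores the reference and adds it to the viewport.
; It then binds to the OnHealthChange dispatcher on the controlled pawn's BPC_CharacterInfo component, though no handler logic appears in this graph.
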(event EventBeginPlay
  (bind _returnvalue (UserInterface|CreateWidget "/Game/ARpgFps/Player/UI/WBP_HUD.WBP_HUD_C"))
  (Variables|Default|SetHUDWidgetRef _returnvalue)
  (UserInterface|Viewport|AddtoViewport (Variables|Default|GetHUDWidgetRef) 0)
  (EventDispatchers|BindEventtoOnHealthChange (Actor|GetComponentbyClass (Pawn|GetControlledPawn (Game|GetPlayerController 0)) "/Game/ARpgFps/Characters/Global/BPC_CharacterInfo.BPC_CharacterInfo_C") (EventDispatchers|CreateEvent (Variables|/Game/ARpgFps/Player/UI/WBP_HUD.WBP_HUD_C|GetW_HealBar (Variables|Default|GetHUDWidgetRef)) :!event SetNewHealth)))

(event Collision|EventActorBeginOverlap
  (params (OtherActor :type Actor%20Object%20Reference)))

(event EventTick
  (params (DeltaSeconds :type Float%20%28single-precision%29)))

(fn ConstructionScript)