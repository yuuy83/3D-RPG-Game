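; Base projectile Blueprint that deals point damage to the actor it hits.
; On BeginPlay, its sphere collision ignores the instigator while moving, so the shooter is not struck by its own shot.
; When ProjectileMovement stops, it applies its base damage to the hit actor, passing the hit result, direction toward that actor and instigator controller.
; The graph does not destroy the projectile after impact.
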(event OnProjectileStop(ProjectileMovement)
  (params (ImpactResult :type Hit%20Result%20Structure%20%28by%20ref%29))
  (bind _hitactor (Collision|BreakHitResult ImpactResult))
  ;[0.15 0.15 0.15 0.5] set damage of projectile
  (Game|Damage|ApplyPointDamage _hitactor (Variables|Default|GetProjectileBaseDamage) (Math|Vector|GetUnitDirection(Vector) (Transformation|GetActorLocation) (Transformation|GetActorLocation _hitactor)) ImpactResult (Game|GetInstigatorController) self))

(event EventBeginPlay
  (Collision|IgnoreActorwhenMoving (Variables|Default|GetSphereCollision) (Game|GetInstigator) true))

(event Collision|EventActorBeginOverlap
  (params (OtherActor :type Actor%20Object%20Reference)))

(event EventTick
  (params (DeltaSeconds :type Float%20%28single-precision%29)))

(fn ConstructionScript)